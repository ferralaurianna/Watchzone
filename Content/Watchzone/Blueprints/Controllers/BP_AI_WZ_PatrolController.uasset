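; AI controller for Watchzone patrol characters that turns perception updates into Blackboard alert states.
; On each target perception update it branches on the stimulus sense class: sight stores the target actor, hearing stores that actor's current location.
; Each branch sets a matching AlertState, with other senses resetting it to the base value.
; It never checks whether the stimulus was successfully sensed, so losing sight is handled like gaining it.
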(event OnTargetPerceptionUpdated(AIPerception)
  (params (Actor :type Actor%20Object%20Reference) (Stimulus :type AI%20Stimulus%20Structure))
  (bind _returnvalue (Class|AIPerceptionSystem|GetSenseClassforStimulus Stimulus))
  (if (== _returnvalue "/Script/AIModule.AISense_Sight")
    (AI|Components|Blackboard|SetValueasObject (Variables|Default|GetBlackboard%20Comp) (Utilities|Name|MakeLiteralName "TargetActor") Actor)
    (AI|Components|Blackboard|SetValueasEnum (Variables|Default|GetBlackboard%20Comp) (Utilities|Name|MakeLiteralName "AlertState") 2)
    (else
      (bind _returnvalue_2 (Class|AIPerceptionSystem|GetSenseClassforStimulus Stimulus))
      (if (== _returnvalue_2 "/Script/AIModule.AISense_Hearing")
        (AI|Components|Blackboard|SetValueasVector (Variables|Default|GetBlackboard%20Comp) (Utilities|Name|MakeLiteralName "TargetLocation") (Transformation|GetActorLocation Actor))
        (AI|Components|Blackboard|SetValueasEnum (Variables|Default|GetBlackboard%20Comp) (Utilities|Name|MakeLiteralName "AlertState") 1)
        (else
          (AI|Components|Blackboard|SetValueasEnum (Variables|Default|GetBlackboard%20Comp) (Utilities|Name|MakeLiteralName "AlertState")))))))

(fn ConstructionScript)